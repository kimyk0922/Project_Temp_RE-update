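; BP_Bed is a bed actor that puts the player to sleep when its box is overlapped.
; The overlap moves the player pawn onto the box with a rotation, calls BP_Player's Sleep and disables input.
; A five-second timer then calls WakeUp, which moves the player to world origin, restores input and sets the mesh's animation to ABP_Manny.
; Respawn and blur-removal helpers exist but are not called here.
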(event `self.Box.OnComponentBeginOverlap`
  (params (OverlappedComponent :type "PrimitiveComponent Object Reference") (OtherActor :type "Actor Object Reference") (OtherComp :type "PrimitiveComponent Object Reference") (OtherBodyIndex :type Integer) (bFromSweep :type Boolean) (SweepResult :type "HitResult Structure (by ref)"))
  (bind _returnvalue (`GameplayStatics.GetPlayerPawn` 0))
  ;[1 1 1 1 15] GoToBed
  (`self.K2_SetActorLocationAndRotation` _returnvalue (`SceneComponent.K2_GetComponentLocation` (`self.Box`)) (struct :`Yaw` -90.0) false false)
  (bind _asbp_player (cast `/Game/Create/GM/BP_Player` _returnvalue))
  (`/Game/Create/GM/BP_Player.Sleep` _asbp_player)
  (`self.DisableInput` _returnvalue (`GameplayStatics.GetPlayerController` 0))
  ;[1 1 1 1 15] WakeUp
  (`KismetSystemLibrary.K2_SetTimer` null "WakeUp" 5.0))

(fn `RemoveBlur`
  (params (Target :type "Widget Object Reference"))
  (`Widget.RemoveFromParent` Target))

(fn `Sleep`)

(fn `UserConstructionScript`)

(fn `WakeUp`
  (bind _returnvalue (`GameplayStatics.GetPlayerPawn` 0))
  (bind _asbp_player (cast `/Game/Create/GM/BP_Player` _returnvalue))
  (`SceneComponent.K2_SetWorldLocation` (`Actor.RootComponent` _asbp_player) (0.0 0.0 0.0) false false)
  (`self.EnableInput` _returnvalue (`GameplayStatics.GetPlayerController` 0))
  (`SkeletalMeshComponent.SetAnimInstanceClass` (`Character.Mesh` _asbp_player) "/Game/Characters/Mannequins/Animations/ABP_Manny.ABP_Manny_C"))

(fn `WakeUp_Spawn`
  (bind _returnvalue (`GameplayStatics.GetPlayerController` 0))
  (`self.K2_DestroyActor` (`GameplayStatics.GetPlayerPawn` 0))
  (bind _returnvalue_2 (`|SpawnActorFromClass` "/Game/Create/GM/BP_Player.BP_Player_C" (`KismetMathLibrary.MakeTransform` (0.0 0.0 0.0)) "Undefined" "MultiplyWithRoot" _returnvalue null))
  (`Controller.Possess` _returnvalue _returnvalue_2))